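; Grid layout actor that spawns a SizeX by SizeY field of GridSpace actors around its location on BeginPlay.
; A 2D grid macro supplies cell centers at BlockSpacing intervals, and each spawned space receives this actor as OwningGrid.
; CreateBoxAtPosition turns generated, offset box geometry into CustomMesh triangles.
; The four-box play-area border that uses it is disconnected, so it never runs.
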(event EventBeginPlay
  ;[1 1 1] Spawn blocks
  (bind _poly_center (Utilities|2DGridExecutionMacro (Variables|Default|GetBlockSpacing) (Transformation|GetActorLocation) (Variables|Default|GetSizeX) (Variables|Default|GetSizeY))
    (:Per%20Poly%20Execution
      (Game|SpawnActorfromClass "/Game/Blueprint/GridSpace_2018-02-11-01-01-39.GridSpace_C" (Math|Conversions|ToTransform(Vector) _poly_center) "Undefined" 0 self 0))))

(fn ConstructionScript)

(fn CreateBoxatPosition
  (params (Box%20Radius :type Vector) (Box%20Position :type Vector) (Custom%20Mesh :type Custom%20Mesh%20Component%20Object%20Reference))
  (bind _triangles (Variables|Default|GetTriangles))
  (bind _vertices (Variables|Default|GetVertices))
  (Utilities|Array|Clear (Variables|Default|GetTriangles))
  (Utilities|Array|Clear (Variables|Default|GetVertices))
  (bind (_vertices_2 _triangles_2) (Class|KismetProceduralMeshLibrary|GenerateBoxMesh Box%20Radius))
  (bind _output_get (Variables|Default|SetBoxTriangles _triangles_2))
  (for (_array_element _array_index) _vertices_2
    (Utilities|Array|SetArrayElem (Variables|Default|GetVertices) _array_index (+ _array_element Box%20Position) true))
  (for _index (range 0 (- (/ (Utilities|Array|Length _output_get) 3) 1))
    (Utilities|Array|Add _triangles (Utilities|Struct|MakeCustomMeshTriangle (Utilities|Array|Get(acopy) _vertices (Utilities|Array|Get(acopy) (Variables|Default|GetBoxTriangles) (* _index 3))) (Utilities|Array|Get(acopy) _vertices (Utilities|Array|Get(acopy) (Variables|Default|GetBoxTriangles) (+ (* _index 3) 1))) (Utilities|Array|Get(acopy) _vertices (Utilities|Array|Get(acopy) (Variables|Default|GetBoxTriangles) (+ (* _index 3) 2)))))
    (Class|CustomMeshComponent|SetCustomMeshTriangles Custom%20Mesh _triangles))
  (return))
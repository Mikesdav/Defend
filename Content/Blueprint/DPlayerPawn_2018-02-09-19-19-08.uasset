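; Player pawn that serves as a touch-driven camera, with drag panning and pinch zoom on a spring arm.
; Touch events store ground hit points and arm length, which Tick uses to move the pawn and scale the clamped arm length.
; Two-finger panning follows the touch midpoint, and the mouse wheel also zooms.
; Older touch and rotation logic is disconnected, and ClampToSize's XY bounds node is unused.
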(event EventBeginPlay)

(event Collision|EventActorBeginOverlap
  (params (OtherActor :type Actor%20Object%20Reference)))

(event EventTick
  (params (DeltaSeconds :type Float%20%28single-precision%29))
  (bind _returnvalue (Game|GetPlayerController 0))
  (bind _returnvalue_2 (Transformation|GetActorLocation))
  (bind _starttouchlocation1 (Variables|Default|GetStartTouchLocation1))
  (bind _touch_2_down (Variables|Default|GetTouch%202%20Down))
  (bind _starttouchlocation2 (Variables|Default|GetStartTouchLocation2))
  (bind _starttouchlocation1_2 (Variables|Default|GetStartTouchLocation1))
  (bind _starttouchlocation2_2 (Variables|Default|GetStartTouchLocation2))
  (bind (_hitresult _returnvalue_3) (Class|PlayerController|GetHitResultUnderFingerbyChannel _returnvalue "Touch1" "TraceTypeQuery1" false))
  (bind (_x _y) (Math|Vector|BreakVector _starttouchlocation2))
  (bind _returnvalue_4 (Math|Vector|Lerp(Vector) _starttouchlocation2_2 _starttouchlocation1 0.5))
  (bind (_x_2 _y_2) (Math|Vector|BreakVector _starttouchlocation2_2))
  (bind (_x_3 _y_3) (Math|Vector|BreakVector _starttouchlocation1))
  (bind (_hitresult_2 _returnvalue_5) (Class|PlayerController|GetHitResultUnderFingerbyChannel _returnvalue "Touch2" "TraceTypeQuery1" false))
  (bind (_x_4 _y_4) (Math|Vector|BreakVector _starttouchlocation1_2))
  (bind _location (Collision|BreakHitResult _hitresult))
  (bind (_x_5 _y_5) (Math|Vector|BreakVector _returnvalue_4))
  (bind _returnvalue_6 (- _x_3 _x_2))
  (bind _returnvalue_7 (- _y_3 _y_2))
  (bind _location_2 (Collision|BreakHitResult _hitresult_2))
  (bind (_x_6 _y_6) (Math|Vector|BreakVector _location_2))
  (bind _returnvalue_8 (Math|Vector|Lerp(Vector) _location_2 _location 0.5))
  (bind _returnvalue_9 (Math|Vector|MakeVector _returnvalue_6 _returnvalue_7 0.0))
  (bind (_x_7 _y_7) (Math|Vector|BreakVector _location))
  (bind (_x_8 _y_8) (Math|Vector|BreakVector _location_2))
  (bind (_x_9 _y_9) (Math|Vector|BreakVector _location))
  (bind _returnvalue_10 (Math|Vector|VectorLengthXY _returnvalue_9))
  (bind (_x_10 _y_10) (Math|Vector|BreakVector _returnvalue_8))
  (bind _returnvalue_11 (- _y_9 _y_8))
  (bind _returnvalue_12 (- _x_9 _x_8))
  (bind _returnvalue_13 (- _x_5 _x_10))
  (bind _returnvalue_14 (- _y_5 _y_10))
  (bind _returnvalue_15 (Math|Vector|MakeVector _returnvalue_12 _returnvalue_11 0.0))
  (bind _returnvalue_16 (Math|Vector|VectorLengthXY _returnvalue_15))
  (bind _returnvalue_17 (Math|Vector|MakeVector _returnvalue_13 _returnvalue_14 0.0))
  (bind _returnvalue_18 (/ _returnvalue_10 _returnvalue_16))
  ;[1 1 1] Comment
  (Utilities|FlowControl|Sequence
    (:then_0
      (if (Math|Boolean|NotEqual(Boolean) (Variables|Default|GetTouch%201%20Down) _touch_2_down)
        (if _touch_2_down
          (Transformation|SetActorLocation (Utilities|ClamptoSize (+ (Transformation|GetActorLocation) (Math|Vector|MakeVector (- _x _x_6) (- _y _y_6) 0.0))) false false)
          (else
            (Transformation|SetActorLocation (Utilities|ClamptoSize (+ (Transformation|GetActorLocation) (Math|Vector|MakeVector (- _x_4 _x_7) (- _y_4 _y_7) 0.0))) false false)))
        (elif _touch_2_down
          (Variables|/Script/Engine.SpringArmComponent|SetTargetArmLength (Variables|Default|GetSpringArm) (Math|Float|Clamp(Float) (* _returnvalue_18 (Variables|Default|GetStartArmLength)) 1e+02 2e+03))
          (Transformation|SetActorLocation (Utilities|ClamptoSize (Math|Vector|Lerp(Vector) _returnvalue_2 (+ _returnvalue_2 _returnvalue_17) 0.8)) false false)
          (Development|PrintString (Utilities|String|Append (Utilities|String|ToString(Vector) _returnvalue_17) "   " (Utilities|String|ToString(Float) _returnvalue_18)) true false "(R=0.000000,G=0.660000,B=1.000000,A=1.000000)" 0.0))))))

(event Input|AxisEvents|InputAxisPinchZoom
  (params (AxisValue :type Float%20%28single-precision%29))
  ;[1 1 1] Camera Zoom
)

(event Input|MouseEvents|MouseWheelUp
  (params (Key :type Key%20Structure))
  (bind _springarm (Variables|Default|GetSpringArm))
  ;[1 1 1] Camera Zoom
  (:Pressed
    (bind _output_get (Variables|/Script/Engine.SpringArmComponent|SetTargetArmLength _springarm (Math|Float|Clamp(Float) (+ (Variables|/Script/Engine.SpringArmComponent|GetTargetArmLength _springarm) (* (Class|Actor|GetInputAxisKeyValue) -25.0)) 1e+02 2e+03)))
    (Development|PrintString (Utilities|String|ToString(Float) _output_get) true false "(R=0.000000,G=0.660000,B=1.000000,A=1.000000)" 0.0)))

(event Input|MouseEvents|MouseWheelDown
  (params (Key :type Key%20Structure))
  (bind _springarm (Variables|Default|GetSpringArm))
  ;[1 1 1] Camera Zoom
  (:Pressed
    (bind _output_get (Variables|/Script/Engine.SpringArmComponent|SetTargetArmLength _springarm (Math|Float|Clamp(Float) (+ (Variables|/Script/Engine.SpringArmComponent|GetTargetArmLength _springarm) (* (Class|Actor|GetInputAxisKeyValue) -25.0)) 1e+02 2e+03)))
    (Development|PrintString (Utilities|String|ToString(Float) _output_get) true false "(R=0.000000,G=0.660000,B=1.000000,A=1.000000)" 0.0)))

(event Input|TouchEvents|Touch1
  (params (Key :type Key%20Structure))
  (bind _returnvalue (Game|GetPlayerController 0))
  (bind (_hitresult _returnvalue_2) (Class|PlayerController|GetHitResultUnderFingerbyChannel _returnvalue "Touch1" "TraceTypeQuery1" false))
  ;[1 1 1] Comment
  (:Pressed
    (bind _output_get (Variables|Default|SetTouch%201%20Down true))
    (if _returnvalue_2
      (Variables|Default|SetStartTouchLocation1 (.Location (Collision|BreakHitResult _hitresult)))
      (Variables|Default|SetStartArmLength (Variables|/Script/Engine.SpringArmComponent|GetTargetArmLength (Variables|Default|GetSpringArm)))))
  (:Released
    (Variables|Default|SetTouch%201%20Down false)
    (if (stale Input|TouchEvents|Touch2 _output_get)
      (Variables|Default|SetStartTouchLocation2 (.Location (Collision|BreakHitResult (.HitResult (Class|PlayerController|GetHitResultUnderFingerbyChannel _returnvalue "Touch2" "TraceTypeQuery1" false))))))))

(event Input|TouchEvents|Touch2
  (params (Key :type Key%20Structure))
  (bind _returnvalue (Game|GetPlayerController 0))
  (bind (_hitresult _returnvalue_2) (Class|PlayerController|GetHitResultUnderFingerbyChannel _returnvalue "Touch2" "TraceTypeQuery1" false))
  ;[1 1 1] Comment
  (:Pressed
    (bind _output_get (Variables|Default|SetTouch%202%20Down true))
    (if _returnvalue_2
      (Variables|Default|SetStartTouchLocation2 (.Location (Collision|BreakHitResult _hitresult)))
      (Variables|Default|SetStartArmLength (Variables|/Script/Engine.SpringArmComponent|GetTargetArmLength (Variables|Default|GetSpringArm)))))
  (:Released
    (Variables|Default|SetTouch%202%20Down false)
    (if (stale Input|TouchEvents|Touch1 _output_get)
      (Variables|Default|SetStartTouchLocation1 (.Location (Collision|BreakHitResult (.HitResult (Class|PlayerController|GetHitResultUnderFingerbyChannel _returnvalue "Touch1" "TraceTypeQuery1" false))))))))

(fn ConstructionScript)